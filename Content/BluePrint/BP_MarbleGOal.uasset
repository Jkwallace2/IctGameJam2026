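; Marble goal trigger that drives target actors when a BP_Marble enters or leaves its box.
; The first entry plays a bell, sends Activate to TargetActors and EnableMessage(false) to the Enable and Disable references; every entry also plays a Ramune sound.
; Exit plays a pop and sends Deactivate through a second DoOnce that activation re-arms.
; The entry DoOnce has no live reset, so activation fires only once.
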(event `self.Box.OnComponentBeginOverlap`
  (params (OverlappedComponent :type "PrimitiveComponent Object Reference") (OtherActor :type "Actor Object Reference") (OtherComp :type "PrimitiveComponent Object Reference") (OtherBodyIndex :type Integer) (bFromSweep :type Boolean) (SweepResult :type "HitResult Structure (by ref)"))
  (bind _targetactors (`self.TargetActors`))
  (cast `/Game/BluePrint/BP_Marble` OtherActor)
  (`|ExecutionSequence`
    (:`then_0`
      (`/Engine/EditorBlueprintResources/StandardMacros.DoOnce` false
        (:`Completed`
          (`GameplayStatics.PlaySound2D` "/Game/Audio/SFX/Jaedon_Wallace_-_Least_of_These_Processed_Foley/03_Toys/Bell_Microwave03.Bell_Microwave03" 1.0 1.0 0.0 null null)
          (message `/Game/MOdels/BarrelInterface.Activate` _targetactors)
          (message `/Game/MOdels/BarrelInterface.Enable` (`self.Enable`) false)
          (message `/Game/MOdels/BarrelInterface.Enable` (`self.Disable`) false)
          (goto _label :!via `Reset`))))
    (:`then_1`
      (`GameplayStatics.PlaySound2D` "/Game/Audio/SoundCues/Collectables/SC_Ramune.SC_Ramune" 1.0 1.0 0.0 null null))))

(event `self.Box.OnComponentEndOverlap`
  (params (OverlappedComponent :type "PrimitiveComponent Object Reference") (OtherActor :type "Actor Object Reference") (OtherComp :type "PrimitiveComponent Object Reference") (OtherBodyIndex :type Integer))
  (cast `/Game/BluePrint/BP_Marble` OtherActor)
  (`/Engine/EditorBlueprintResources/StandardMacros.DoOnce` false :!label _label
    (:`Completed`
      (`GameplayStatics.PlaySound2D` "/Game/Audio/SFX/WallaceToySFX/00_Toys/Toy_Pop3.Toy_Pop3" 1.0 1.0 0.0 null null)
      (message `/Game/MOdels/BarrelInterface.Deactivate` (`self.TargetActors`)))))

(fn `UserConstructionScript`)