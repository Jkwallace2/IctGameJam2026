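; BP_Barrel is a barrel actor that spins around its local roll axis at an externally set speed.
; BeginPlay caches the root's world location as Origin and the bounds' Z extent as Radius.
; AddRotationSpeed overwrites RotateAmount, which Tick applies as a per-frame roll without delta-time scaling before storing the resulting roll in Rotation.
; GetSpeedPlease is a stub that always returns zero.
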(event `self.ReceiveBeginPlay`
  (set `self.Origin` (`SceneComponent.K2_GetComponentLocation` (`self.DefaultSceneRoot`)))
  (set `self.Radius` (.z (`.BoxExtent` (`self.GetActorBounds` false)))))

(event `self.ReceiveTick`
  (params (DeltaSeconds :type "Float (single-precision)"))
  (`self.K2_AddActorLocalRotation` (`KismetMathLibrary.MakeRotator` (`self.Rotate Amount`)))
  (set `self.Rotation` (.roll (`self.K2_GetActorRotation`))))

(event `/Game/MOdels/BarrelInterface.AddRotationSpeed`
  (params (Speed :type "Float (double-precision)"))
  (set `self.Rotate Amount` Speed))

(fn `GetSpeedPlease`
  (params (Speed :type "Float (double-precision)"))
  (returns (Speedout :type "Float (double-precision)"))
  (return 0.0))

(fn `UserConstructionScript`)