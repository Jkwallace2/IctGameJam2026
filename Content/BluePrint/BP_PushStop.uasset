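; BP_PushStop is a trigger that halts a BP_PushTHing entering its box.
; Box overlap sends StopMessage to the pusher with its Reverse value and both stop flags set, then clears those flags when the overlap ends.
; A DoOnce plays a hatch-close sound on entry and re-arms on exit.
; GetSpeedPlease only returns zero.
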(event `self.Box.OnComponentBeginOverlap`
  (params (OverlappedComponent :type "PrimitiveComponent Object Reference") (OtherActor :type "Actor Object Reference") (OtherComp :type "PrimitiveComponent Object Reference") (OtherBodyIndex :type Integer) (bFromSweep :type Boolean) (SweepResult :type "HitResult Structure (by ref)"))
  (bind _asbp_push_thing (cast `/Game/BluePrint/BP_PushTHing` OtherActor))
  (message `/Game/MOdels/BarrelInterface.Stop` _asbp_push_thing (`self.Reverse`) true true)
  (`/Engine/EditorBlueprintResources/StandardMacros.DoOnce` false :!label _label
    (:`Completed`
      (`GameplayStatics.PlaySoundAtLocation` "/Game/Audio/SFX/WallaceToySFX/00_Toys/Toy_Hatch_Close.Toy_Hatch_Close" (`self.K2_GetActorLocation`) (struct) 1.0 1.0 0.0 null null null null))))

(event `self.Box.OnComponentEndOverlap`
  (params (OverlappedComponent :type "PrimitiveComponent Object Reference") (OtherActor :type "Actor Object Reference") (OtherComp :type "PrimitiveComponent Object Reference") (OtherBodyIndex :type Integer))
  (bind _asbp_push_thing (cast `/Game/BluePrint/BP_PushTHing` OtherActor))
  (message `/Game/MOdels/BarrelInterface.Stop` _asbp_push_thing (`self.Reverse`) false false)
  (goto _label :!via `Reset`))

(fn `GetSpeedPlease`
  (params (Speed :type "Float (double-precision)"))
  (returns (Speedout :type "Float (double-precision)"))
  (return 0.0))

(fn `UserConstructionScript`)