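; BP_TrapDoor is a trap door that breaks away when activated and restores itself a few seconds later.
; Activate calls Open, which plays wood-break effects at the door and disables the mesh's collision and visibility.
; A retriggerable delay then calls Deactivate, also a standalone event, which restores the door with an explosion effect and pickup sound.
; GetSpeedPlease is a stub that returns zero.
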(event `Open`
  (`NiagaraFunctionLibrary.SpawnSystemAtLocation` "/Game/LeastOfThese/VFX/Destruction/NS_WoodBreak.NS_WoodBreak" (`KismetSystemLibrary.GetComponentBounds` (`self.SM_ToyDoors_KU_Door1`)))
  (`GameplayStatics.PlaySoundAtLocation` "/Game/Audio/SFX/Phisics/Wood/SC_WoodBreak.SC_WoodBreak" (`self.K2_GetActorLocation`) (struct) 1.0 1.0 0.0 null null null null)
  (`PrimitiveComponent.SetCollisionEnabled` (`self.SM_ToyDoors_KU_Door1`) "NoCollision")
  (`SceneComponent.SetVisibility` (`self.SM_ToyDoors_KU_Door1`) false false)
  (`KismetSystemLibrary.RetriggerableDelay` 4.0)
  (`/Game/MOdels/BarrelInterface.Deactivate`))

(event `self.Deactivate`
  (`NiagaraFunctionLibrary.SpawnSystemAtLocation` "/Game/LeastOfThese/VFX/NS_Explosion.NS_Explosion" (`KismetSystemLibrary.GetComponentBounds` (`self.SM_ToyDoors_KU_Door1`)))
  (`GameplayStatics.PlaySoundAtLocation` "/Game/Audio/SFX/WallaceToySFX/05_GameSounds/Game_Pickup.Game_Pickup" (`self.K2_GetActorLocation`) (struct) 1.0 1.0 0.0 null null null null)
  (`PrimitiveComponent.SetCollisionEnabled` (`self.SM_ToyDoors_KU_Door1`) "QueryAndPhysics")
  (`SceneComponent.SetVisibility` (`self.SM_ToyDoors_KU_Door1`) true false))

(event `self.Activate`
  (`self.Open`))

(fn `GetSpeedPlease`
  (params (Speed :type "Float (double-precision)"))
  (returns (Speedout :type "Float (double-precision)"))
  (return 0.0))

(fn `UserConstructionScript`)