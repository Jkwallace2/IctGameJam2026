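; Player goal actor that acts as a one-time trigger and soft checkpoint when the player pawn overlaps its box.
; The first overlap plays impact and prize sounds, messages TargetActors to activate, sends EnableMessage false to Enable and true to Disable, and turns the cylinder green.
; Every player overlap also plays a sound and sends the pawn a soft checkpoint just above the goal mesh.
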(event `self.Box.OnComponentBeginOverlap`
  (params (OverlappedComponent :type "PrimitiveComponent Object Reference") (OtherActor :type "Actor Object Reference") (OtherComp :type "PrimitiveComponent Object Reference") (OtherBodyIndex :type Integer) (bFromSweep :type Boolean) (SweepResult :type "HitResult Structure (by ref)"))
  (if (== OtherActor (`GameplayStatics.GetPlayerPawn` 0))
    (`|ExecutionSequence`
      (:`then_0`
        (`/Engine/EditorBlueprintResources/StandardMacros.DoOnce` false
          (:`Completed`
            (`GameplayStatics.PlaySound2D` "/Game/Audio/SFX/Jaedon_Wallace_-_Foley_2nd_Batch/SoftMarbleImpact.SoftMarbleImpact" 1.0 1.0 0.0 null null)
            (message `/Game/MOdels/BarrelInterface.Activate` (`self.TargetActors`))
            (message `/Game/MOdels/BarrelInterface.Enable` (`self.Enable`) false)
            (message `/Game/MOdels/BarrelInterface.Enable` (`self.Disable`) true)
            (`PrimitiveComponent.SetMaterial` (`self.Cylinder`) 0 "/Game/LeastOfThese/Materials/Shaders/MI_CollectGreen.MI_CollectGreen")
            (`GameplayStatics.PlaySound2D` "/Game/Audio/SFX/Jaedon_Wallace_-_Foley_2nd_Batch/Prize_ObjectHit2.Prize_ObjectHit2" 3.0 0.9 0.0 null null))))
      (:`then_1`
        (`GameplayStatics.PlaySound2D` "/Game/Audio/SoundCues/Collectables/SC_Ramune.SC_Ramune" 1.0 1.0 0.0 null null)
        (message `/Game/StateTreePlayer/FirstPerson/Blueprints/BPI_WorldToPlayerInteraction.SoftCheckpoint` (`GameplayStatics.GetPlayerPawn` 0) (`KismetMathLibrary.Conv_VectorToTransform` (+ (`SceneComponent.K2_GetComponentLocation` (`self.SM_MarbleGoal`)) (0.0 0.0 100.0))))))))

(fn `UserConstructionScript`)