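; BP_MarbleSpawner is an activatable launcher that replaces every BP_Marble in the level with a fresh one spawned at its root.
; Activate passes a DoOnce, calls DeletePlease on existing marbles, spawns after a short delay, then re-arms after a cooldown.
; Enable or StartDisabled sets the Disabled flag, which limits Activate to a click sound.
; Material swaps on the mesh show ready, cooling-down and disabled states, with sound cues.
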(event `self.ReceiveBeginPlay`
  (if (`self.StartDisabled`)
    (set `self.Disabled` true)
    (`PrimitiveComponent.SetMaterial` (`self.StaticMesh`) 1 "/Game/LeastOfThese/Materials/Marbles/MI_MarbleBlack.MI_MarbleBlack")))

(event `/Game/MOdels/BarrelInterface.Activate`
  (bind _returnvalue (`self.K2_GetActorLocation`))
  (if (`self.Disabled`)
    (`GameplayStatics.PlaySoundAtLocation` "/Game/Audio/SFX/WallaceToySFX/00_Toys/Toy_Click_Up.Toy_Click_Up" _returnvalue (struct) 1.0 1.0 0.0 null null null null)
    (`PrimitiveComponent.SetMaterial` (`self.StaticMesh`) 1 "/Game/LeastOfThese/Materials/Marbles/MI_MarbleBlack.MI_MarbleBlack")
    (else
      (`GameplayStatics.PlaySoundAtLocation` "/Game/Audio/SFX/WallaceToySFX/00_Toys/Toy_RevSpin.Toy_RevSpin" _returnvalue (struct) 1.0 1.0 0.0 null null null null)
      (`/Engine/EditorBlueprintResources/StandardMacros.DoOnce` false :!label _label
        (:`Completed`
          (bind _outactors (`GameplayStatics.GetAllActorsOfClass` "/Game/BluePrint/BP_Marble.BP_Marble_C"))
          (`/Game/BluePrint/BP_Marble.DeletePlease` _outactors)
          (`PrimitiveComponent.SetMaterial` (`self.StaticMesh`) 1 "/Game/LeastOfThese/Materials/Shaders/MI_CollectRed.MI_CollectRed")
          (`GameplayStatics.PlaySoundAtLocation` "/Game/Audio/SFX/WallaceToySFX/00_Toys/Toy_GrenadeLauncher.Toy_GrenadeLauncher" _returnvalue (struct) 3.0 1.0 0.0 null null null null)
          (`KismetSystemLibrary.Delay` 0.3)
          (`|SpawnActorFromClass` "/Game/BluePrint/BP_Marble.BP_Marble_C" (`KismetMathLibrary.Conv_VectorToTransform` (`SceneComponent.K2_GetComponentLocation` (`self.DefaultSceneRoot`))) "Undefined" "MultiplyWithRoot" null null)
          (`KismetSystemLibrary.RetriggerableDelay` 5.0)
          (`GameplayStatics.PlaySoundAtLocation` "/Game/Audio/SFX/Jaedon_Wallace_-_Foley_2nd_Batch/Marble_Pickup3.Marble_Pickup3" (`self.K2_GetActorLocation`) (struct) 1.0 1.0 0.0 null null null null)
          (if (`self.Disabled`)
            (`PrimitiveComponent.SetMaterial` (`self.StaticMesh`) 1 "/Game/LeastOfThese/Materials/Marbles/MI_MarbleBlack.MI_MarbleBlack")
            (goto _label :!via `Reset`)
            (else
              (`PrimitiveComponent.SetMaterial` (`self.StaticMesh`) 1 "/Game/LeastOfThese/Materials/Shaders/MI_CollectGreen.MI_CollectGreen")
              (goto _label :!via `Reset`))))))))

(event `/Game/MOdels/BarrelInterface.UseBUtton`)

(event `/Game/MOdels/BarrelInterface.Enable`
  (params (Disable :type Boolean))
  (bind _output_get (set `self.Disabled` Disable))
  (if _output_get
    (`PrimitiveComponent.SetMaterial` (`self.StaticMesh`) 1 "/Game/LeastOfThese/Materials/Marbles/MI_MarbleBlack.MI_MarbleBlack")
    (`GameplayStatics.PlaySoundAtLocation` "/Game/Audio/SFX/WallaceToySFX/00_Toys/Toy_Click_Up.Toy_Click_Up" (`self.K2_GetActorLocation`) (struct) 1.0 1.0 0.0 null null null null)
    (else
      (`PrimitiveComponent.SetMaterial` (`self.StaticMesh`) 1 "/Game/LeastOfThese/Materials/Shaders/MI_CollectGreen.MI_CollectGreen")
      (goto _label :!via `Reset`))))

(fn `GetSpeedPlease`
  (params (Speed :type "Float (double-precision)"))
  (returns (Speedout :type "Float (double-precision)"))
  (return 0.0))

(fn `UserConstructionScript`)