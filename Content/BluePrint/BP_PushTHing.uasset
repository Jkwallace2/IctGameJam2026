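; Pushable object Blueprint whose mesh slides along world X when pushed or pulled.
; Push projects the horizontal push vector onto the actor's forward, scales it by Pushspeed, negates it for pulls, shifts TargetPosition and plays a pitched sound.
; Tick eases the mesh toward that target with VInterpTo while CanMove is set.
; Stop toggles CanMoveX, identically in both X branches, and can freeze the target at the current position.
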(event `self.ReceiveTick`
  (params (DeltaSeconds :type "Float (single-precision)"))
  (bind _returnvalue (`SceneComponent.K2_GetComponentLocation` (`self.StaticMesh`)))
  (if (`self.canMove`)
    (`SceneComponent.K2_SetWorldLocation` (`self.StaticMesh`) (`KismetMathLibrary.VInterpTo` _returnvalue (+ (* _returnvalue (0.0 1.0 1.0)) (`KismetMathLibrary.MakeVector` (`self.TargetPosition`))) DeltaSeconds 3.0) false false)))

(event `/Game/MOdels/BarrelInterface.Push`
  (params (PushVec :type "Vector Structure") (Pull :type Boolean))
  (bind _returnvalue (* (`KismetMathLibrary.Dot_VectorVector` (* PushVec (1.0 1.0 0.0)) (* (`self.GetActorForwardVector`) (1.0 1.0 0.0))) (`self.Pushspeed`)))
  (bind _returnvalue_2 (select `bool` Pull :`false` _returnvalue :`true` (* _returnvalue -1.0)))
  (if (and (`self.Can MoveX-`) (< _returnvalue_2 0.0))
    (set `self.TargetPosition` (+ (`self.TargetPosition`) _returnvalue_2) :!label _label)
    (`GameplayStatics.PlaySound2D` "/Game/Audio/SFX/Jaedon_Wallace_-_Foley_2nd_Batch/Marble_Drop.Marble_Drop" 1.0 (select `bool` Pull :`false` 0.7 :`true` 0.6) 0.125 "/Game/Audio/SoundCues/SoundCon_SmalMultitiudes.SoundCon_SmalMultitiudes" null)
    (elif (and (> _returnvalue_2 0.0) (`self.CanMoveX+`))
      (goto _label))))

(event `/Game/MOdels/BarrelInterface.Stop`
  (params (`X+` :type Boolean) (Stop :type Boolean) (StopMovement :type Boolean))
  (bind _returnvalue_x (`KismetMathLibrary.BreakVector` (`SceneComponent.K2_GetComponentLocation` (`self.StaticMesh`))))
  (if `X+`
    (set `self.CanMoveX+` (!= Stop true))
    (else
      (set `self.Can MoveX-` (!= Stop true))))
  (if StopMovement
    (set `self.TargetPosition` _returnvalue_x)))

(fn `GetSpeedPlease`
  (params (Speed :type "Float (double-precision)"))
  (returns (Speedout :type "Float (double-precision)"))
  (return 0.0))

(fn `UserConstructionScript`
  (bind _output_get (set `self.OriginX` (.x (`SceneComponent.K2_GetComponentLocation` (`self.StaticMesh`)))))
  (set `self.TargetPosition` _output_get))