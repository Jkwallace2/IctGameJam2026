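; A moving barrel actor whose travel along world Y is tied to its rotation angle, as in rolling without slipping.
; The construction script runs the parent's, then caches Radius from the Cylinder's Z bounds extent.
; The CHildRotation event converts Rotation to arc length and sweeps Scene to that offset from Origin.
; BeginPlay and overlap events are disabled, and the StartLocation and EndLocation placement nodes never run.
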(event `self.CHildRotation`
  (`SceneComponent.K2_SetWorldLocation` (`self.Scene`) (+ (`self.Origin`) (`KismetMathLibrary.MakeVector` 0.0 (* (`self.Radius`) (`KismetMathLibrary.DegreesToRadians` (`self.Rotation`))))) true false))

(fn `UserConstructionScript`
  (`parent.UserConstructionScript`)
  (set `self.Radius` (.z (`.BoxExtent` (`KismetSystemLibrary.GetComponentBounds` (`self.Cylinder`))))))