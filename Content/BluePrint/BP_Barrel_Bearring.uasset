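; BP_Barrel_Bearring is a rotating barrel bearing actor with a rolling sound.
; AddRotationSpeed adds the given speed to an accumulated angle, sets it as the root's world X roll and calls CHildRotation; UpdateCHildren reapplies that angle.
; Each call also keeps the roll audio alive, scaling volume by absolute speed once playing.
; A DoOnce starts the sound, and a half-second retriggerable delay stops it when calls cease.
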(event `/Game/MOdels/BarrelInterface.UpdateCHildren`
  (`SceneComponent.K2_SetWorldRotation` (`self.DefaultSceneRoot`) (`KismetMathLibrary.MakeRotator` (`self.Rotation`)) false false))

(event `/Game/MOdels/BarrelInterface.AddRotationSpeed`
  (params (Speed :type "Float (double-precision)"))
  (bind _roll_objectroll (`self.Roll_ObjectRoll`))
  (bind _roll_objectroll_2 (`self.Roll_ObjectRoll`))
  (set `self.Rotate Amount` Speed)
  (`|ExecutionSequence`
    (:`then_0`
      (if (`self.isPlayingaudio`)
        (`AudioComponent.SetVolumeMultiplier` (`self.Roll_ObjectRoll`) (* (`KismetMathLibrary.Abs` Speed) 2.0))
        (else
          (`/Engine/EditorBlueprintResources/StandardMacros.DoOnce` false :!label _label
            (:`Completed`
              (set `self.isPlayingaudio` true)
              (`ActorComponent.Activate` _roll_objectroll true)
              (`AudioComponent.Play` _roll_objectroll 0.0)))))
      (`KismetSystemLibrary.RetriggerableDelay` 0.5)
      (`|ExecutionSequence`
        (:`then_0`
          (goto _label :!via `Reset`))
        (:`then_1`
          (set `self.isPlayingaudio` false)
          (`AudioComponent.Stop` _roll_objectroll_2)
          (`ActorComponent.Deactivate` _roll_objectroll_2))))
    (:`then_1`
      (`self.CHildRotation`)
      (bind _output_get (set `self.Rotation` (+ (`self.Rotation`) (`self.Rotate Amount`))))
      (`SceneComponent.K2_SetWorldRotation` (`self.DefaultSceneRoot`) (`KismetMathLibrary.MakeRotator` _output_get) false false))))

(event `CustomEvent_1`)

(fn `UserConstructionScript`
  (`parent.UserConstructionScript`))