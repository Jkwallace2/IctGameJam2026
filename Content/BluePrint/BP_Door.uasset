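; BP_Door is a double door that swings open and closed, playing a sound each way, and can start open.
; A Timeline drives the two door meshes in opposite yaw to nearly 90 degrees and reverses to close.
; Activate opens it, Deactivate closes it when KeePOpen is true, and Enable closes it when its Disable flag is true.
; GetSpeedPlease is a stub returning zero.
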(event `self.ReceiveBeginPlay`
  (if (`self.StartOpen`)
    (`self.Open`)))

(event `Open`
  (`GameplayStatics.PlaySoundAtLocation` "/Game/Audio/SoundCues/Collectables/SC_Ramune.SC_Ramune" (`self.K2_GetActorLocation`) (struct) 2.0 1.0 0.0 null null null null)
  (bind (_direction _newtrack_0) (`Timeline|Timeline` :!label _label)
    (:`Update`
      (bind _returnvalue (`KismetMathLibrary.Lerp` 0.0 89.9 _newtrack_0))
      (`SceneComponent.K2_SetRelativeRotation` (`self.SM_ToyDoors_KU_Door`) (`KismetMathLibrary.MakeRotator` 0.0 0.0 _returnvalue) false false)
      (`SceneComponent.K2_SetRelativeRotation` (`self.SM_ToyDoors_KU_Door1`) (`KismetMathLibrary.MakeRotator` 0.0 0.0 (* _returnvalue -1.0)) false false))))

(event `/Game/MOdels/BarrelInterface.Deactivate`
  (if (`self.KeePOpen`)
    (`self.CLose` :!label _label_2)))

(event `CLose`
  (`GameplayStatics.PlaySoundAtLocation` "/Game/Audio/SoundCues/SC_PlayerHurt.SC_PlayerHurt" (`self.K2_GetActorLocation`) (struct) 2.0 1.0 0.0 null null null null)
  (goto _label :!via `Reverse`))

(event `/Game/MOdels/BarrelInterface.Enable`
  (params (Disable :type Boolean))
  (if Disable
    (goto _label_2)))

(event `/Game/MOdels/BarrelInterface.Activate`
  (`self.Open`))

(fn `GetSpeedPlease`
  (params (Speed :type "Float (double-precision)"))
  (returns (Speedout :type "Float (double-precision)"))
  (return 0.0))

(fn `UserConstructionScript`)