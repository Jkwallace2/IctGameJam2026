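; BP_Barrel_Child is a barrel Blueprint child that turns a rotation value into straight-line movement along world Y.
; The CHildRotation event moves the root to Origin offset by Radius times the rotation in radians, the arc length of a rolling body.
; After running the parent's script, the construction script places Start and End at their configured Y offsets from Origin.
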(event `self.CHildRotation`
  (`SceneComponent.K2_SetWorldLocation` (`self.DefaultSceneRoot`) (+ (`self.Origin`) (`KismetMathLibrary.MakeVector` 0.0 (* (`self.Radius`) (`KismetMathLibrary.DegreesToRadians` (`self.Rotation`))))) false false))

(fn `UserConstructionScript`
  (`parent.UserConstructionScript`)
  (`SceneComponent.K2_SetWorldLocation` (`self.Start`) (+ (`self.Origin`) (`KismetMathLibrary.MakeVector` 0.0 (`self.StartLocation`))) false false)
  (`SceneComponent.K2_SetWorldLocation` (`self.End`) (+ (`self.Origin`) (`KismetMathLibrary.MakeVector` 0.0 (`self.EndLocation`))) false false))