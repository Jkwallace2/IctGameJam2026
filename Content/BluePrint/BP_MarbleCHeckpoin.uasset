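; BP_MarbleCHeckpoin is a one-shot checkpoint actor for the marble.
; The first BP_Marble overlap of its box plays a bell sound and turns one checkpoint mesh material green.
; It then sends ActivateMessage to TargetActors and toggles other targets through EnableMessage, passing false to TargetEnable and true to TargetDisable, the reverse of what their names suggest.
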(event `CHeckpoint is go`
  (`GameplayStatics.PlaySoundAtLocation` "/Game/Audio/SFX/WallaceToySFX/03_Bells/Bell_Death.Bell_Death" (`self.K2_GetActorLocation`) (struct) 1.0 1.0 0.0 null null null null)
  (`PrimitiveComponent.SetMaterial` (`self.SM_CHeckpoint`) 1 "/Game/LeastOfThese/Materials/Shaders/MI_CollectGreen.MI_CollectGreen"))

(event `self.Box.OnComponentBeginOverlap`
  (params (OverlappedComponent :type "PrimitiveComponent Object Reference") (OtherActor :type "Actor Object Reference") (OtherComp :type "PrimitiveComponent Object Reference") (OtherBodyIndex :type Integer) (bFromSweep :type Boolean) (SweepResult :type "HitResult Structure (by ref)"))
  (cast `/Game/BluePrint/BP_Marble` OtherActor)
  (`/Engine/EditorBlueprintResources/StandardMacros.DoOnce` false
    (:`Completed`
      (`self.CHeckpoint is go`)
      (message `/Game/MOdels/BarrelInterface.Activate` (`self.TargetActors`))
      (message `/Game/MOdels/BarrelInterface.Enable` (`self.TargetEnable`) false)
      (message `/Game/MOdels/BarrelInterface.Enable` (`self.TargetDisable`) true))))

(fn `UserConstructionScript`)