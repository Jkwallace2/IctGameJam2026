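; Footstep effect actor that detects the surface at a step and sets up the location and rotation for its impact effect.
; GetInfo line-traces down or along the actor's forward vector, depending on UseZVector, ignoring the instigator.
; A hit passes the physical material to BreakKnownPhysMats, then calls Execute after a short delay; a miss destroys the actor.
; A character-specific sound switch on FootInfo is present but never runs.
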(event `self.GetInfo`
  (bind _tracerange (`self.TraceRange`))
  (bind _returnvalue (`SceneComponent.K2_GetComponentLocation` (`self.DefaultSceneRoot`)))
  (if (`self.UseZVector`)
    (set `self.UseXVectorForDecal` false))
  (bind (_outhit _returnvalue_2) (`KismetSystemLibrary.LineTraceSingleByProfile` _returnvalue (+ _returnvalue (`KismetMathLibrary.SelectVector` (* (0.0 0.0 -1.0) _tracerange) (* (`self.GetActorForwardVector`) _tracerange) (`self.UseZVector`))) "BlockAll" false (`|MakeArray` (`self.GetInstigator`) :!type "Actor Object Reference") "None" true (struct :`R` 0.239163 :`B` 1.0 :`A` 1.0) (struct :`R` 1.0 :`B` 0.036416 :`A` 1.0) 15.0))
  (if _returnvalue_2
    (bind (_bblockinghit _binitialoverlap _time _distance _location _impactpoint _normal _impactnormal _physmat) (`GameplayStatics.BreakHitResult` _outhit))
    (set `self.SoundLocation` _impactpoint)
    (set `self.SoundRotation` (`KismetMathLibrary.SelectRotator` (`KismetMathLibrary.ComposeRotators` (`KismetMathLibrary.Conv_VectorToRotator` (`SceneComponent.GetForwardVector` (`self.DefaultSceneRoot`))) (struct :`Yaw` 90.0)) (`KismetMathLibrary.Conv_VectorToRotator` _normal) (`self.UseZVector`)))
    (`self.BreakKnownPhysMats` _physmat)
    ; HeelThenToe
    (`KismetSystemLibrary.Delay` 0.2)
    (`self.Execute`)
    (else
      (`self.K2_DestroyActor`))))

(fn `UserConstructionScript`
  (`parent.UserConstructionScript`))