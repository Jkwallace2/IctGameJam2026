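; BP_Elevator is an elevator actor that moves its static mesh along a spline.
; Activate fires Fuse to play a Timeline forward when GetActorIsThinking is true; Deactivate fires UnFuse to reverse it.
; Timeline progress scales the spline length to set mesh position, with an attached elevator sound stopped on finish.
; DoOnce gates block repeated triggers until the Timeline finishes and resets both.
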(event `Fuse`
  (bind _spline (`self.Spline`))
  (`/Engine/EditorBlueprintResources/StandardMacros.DoOnce` false :!label _label
    (:`Completed`
      (bind _returnvalue (`GameplayStatics.SpawnSoundAttached` "/Game/Audio/SoundCues/SC_Elevator.SC_Elevator" (`self.StaticMesh`) "None" (0.0 0.0 0.0) (struct) "KeepRelativeOffset" false 1.0 1.0 0.0 null null))
      (set `self.NewVar_0` _returnvalue)
      (bind (_direction _fuse) (`Timeline|Timeline` :!label _label_2)
        (:`Update`
          (`SceneComponent.K2_SetRelativeLocation` (`self.StaticMesh`) (`SplineComponent.GetLocationAtDistanceAlongSpline` _spline (* _fuse (`SplineComponent.GetSplineLength` _spline)) "Local") false false))
        (:`Finished`
          (if (`KismetSystemLibrary.IsValid` (`self.NewVar_0`))
            (`AudioComponent.Stop` _returnvalue)
            (`AudioComponent.Stop` (`self.NewVar_0`)))
          (`self.reset`))))))

(event `UnFuse`
  (`/Engine/EditorBlueprintResources/StandardMacros.DoOnce` false :!label _label_3
    (:`Completed`
      (bind _returnvalue (`GameplayStatics.SpawnSoundAttached` "/Game/Audio/SoundCues/SC_Elevator.SC_Elevator" (`self.StaticMesh`) "None" (0.0 0.0 0.0) (struct) "KeepRelativeOffset" false 1.0 1.0 0.0 null null))
      (set `self.NewVar_0` _returnvalue)
      (goto _label_2 :!via `Reverse`))))

(event `reset`
  (`|ExecutionSequence`
    (:`then_0`
      (goto _label :!via `Reset`))
    (:`then_1`
      (goto _label_3 :!via `Reset`))))

(fn `Activate`
  (returns (Successful :type Boolean))
  (if (`self.GetActorIsThinking`)
    (`self.Fuse`)
    (return true)
    (else
      (return false))))

(fn `Deactivate`
  (returns (Successful :type Boolean))
  (`self.UnFuse`)
  (return false))

(fn `UserConstructionScript`
  (`parent.UserConstructionScript`))