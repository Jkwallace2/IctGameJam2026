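; Base spline actor that tiles a chosen static mesh along its spline as spline mesh components, built in the construction script.
; Spline length is divided by SectionLength (optionally derived from actor X scale); MustBeFullLength drops the leftover partial section.
; Each segment samples position, tangent and scale by distance, clamping tangent size to section length.
; Segments receive configurable collision and distance field lighting; no runtime logic.
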(fn `GetendPos/Tan`
  (params (Index :type Integer))
  (returns (Position :type "Vector Structure") (Tangent :type "Vector Structure") (Scale :type "Vector Structure"))
  (bind _spline (`self.Spline`))
  (bind _returnvalue (* (+ Index 1) (`self.Section Length`)))
  (return (`SplineComponent.GetLocationAtDistanceAlongSpline` _spline _returnvalue "Local") (`KismetMathLibrary.ClampVectorSize` (`SplineComponent.GetTangentAtDistanceAlongSpline` _spline _returnvalue "Local") 0.0 (`self.Section Length`)) (`SplineComponent.GetScaleAtDistanceAlongSpline` _spline _returnvalue)))

(fn `GetStartPos/Tan`
  (params (Index :type Integer))
  (returns (Position :type "Vector Structure") (Tangent :type "Vector Structure") (Scale :type "Vector Structure"))
  (bind _spline (`self.Spline`))
  (bind _returnvalue (* Index (`self.Section Length`)))
  (return (`SplineComponent.GetLocationAtDistanceAlongSpline` _spline _returnvalue "Local") (`KismetMathLibrary.ClampVectorSize` (`SplineComponent.GetTangentAtDistanceAlongSpline` _spline _returnvalue "Local") 0.0 (`self.Section Length`)) (`SplineComponent.GetScaleAtDistanceAlongSpline` _spline _returnvalue)))

(fn `UserConstructionScript`
  (bind _returnvalue_x (`KismetMathLibrary.BreakVector` (`self.GetActorScale3D`)))
  (if (`self.AllowScaling`)
    (set `self.Section Length` (* _returnvalue_x 100.0)))
  (if (`self.MustBeFullLength`)
    (for _index (range (`KismetMathLibrary.FTrunc` (/ (`SplineComponent.GetSplineLength` (`self.Spline`)) (`self.Section Length`))))
      (set `self.LoopIndex` _index)
      (bind _returnvalue (`AddComponent|NODE_AddSplineMeshComponent-0` :!label _label))
      (`StaticMeshComponent.SetStaticMesh` _returnvalue (`self.New Mesh`))
      (`StaticMeshComponent.SetDistanceFieldSelfShadowBias` _returnvalue 0.5)
      (`PrimitiveComponent.SetAffectDistanceFieldLighting` _returnvalue true)
      (`SplineMeshComponent.SetForwardAxis` _returnvalue "X" true)
      (bind (_position _tangent _scale) (`self.GetStartPos/Tan` (`self.LoopIndex`)))
      (bind (_position_2 _tangent_2 _scale_2) (`self.GetendPos/Tan` (`self.LoopIndex`)))
      (`SplineMeshComponent.SetStartAndEnd` _returnvalue _position _tangent _position_2 _tangent_2 true)
      (`SplineMeshComponent.SetStartAndEnd` _returnvalue _position _tangent _position_2 _tangent_2 true)
      (`SplineMeshComponent.SetStartScale` _returnvalue (`KismetMathLibrary.MakeVector2D` (.y _scale) (.z _scale)) true)
      (`SplineMeshComponent.SetEndScale` _returnvalue (`KismetMathLibrary.MakeVector2D` (.y _scale_2) (.z _scale_2)) true)
      (`PrimitiveComponent.SetCollisionEnabled` _returnvalue (`self.CollisionType`)))
    (else
      (for _index_2 (range (+ (`KismetMathLibrary.FTrunc` (/ (`SplineComponent.GetSplineLength` (`self.Spline`)) (`self.Section Length`))) 1))
        (set `self.LoopIndex` _index_2)
        (goto _label)))))