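; BP_Sign is a readable sign that shows its text as player dialogue when the player stands in front of it.
; LookTrace compares the player's eye position to LookTrigger, using range and a dot product against the trigger's facing rather than a line trace.
; It sends a brief dialogue message to player 0 (singleplayer only), fading opacity with distance.
; The construction script copies the same Text onto the TextRender.
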(event `/Game/StateTreePlayer/FirstPerson/Blueprints/BPI_WorldToPlayerInteraction.LookTrace`
  (bind _looktrigger (`self.LookTrigger`))
  (bind _returnvalue (`SceneComponent.K2_GetComponentLocation` _looktrigger))
  (bind _outlocation (`self.GetActorEyesViewPoint` (`GameplayStatics.GetPlayerPawn` 0)))
  (bind _returnvalue_2 (`KismetMathLibrary.Vector_Distance` _returnvalue _outlocation))
  (if (< _returnvalue_2 (`self.MaxRange`))
    (if (> (`KismetMathLibrary.Dot_VectorVector` (`KismetMathLibrary.Normal` (- _returnvalue _outlocation)) (* (`SceneComponent.GetForwardVector` _looktrigger) (-1.0 -1.0 -1.0))) (`self.ViewingAngle`))
      (message `/Game/StateTreePlayer/FirstPerson/Blueprints/BPI_WorldToPlayerInteraction.Diolauge` (`GameplayStatics.GetPlayerPawn` 0) (make `/Game/LeastOfThese/DataTables/Structures/Struct_Dialogue` "SIGN" (`self.Text`) 0.002 0.0 false (`KismetMathLibrary.MapRangeClamped` _returnvalue_2 100.0 (`self.MaxRange`) 1.0))))))

(fn `UserConstructionScript`
  (`parent.UserConstructionScript`)
  (`TextRenderComponent.K2_SetText` (`self.TextRender`) (`self.Text`)))