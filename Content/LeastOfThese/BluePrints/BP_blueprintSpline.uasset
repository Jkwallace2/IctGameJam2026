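; Spline actor that spawns instances of a chosen Blueprint class at SectionLength intervals along its spline, oriented to the tangent.
; ChildStartThinking or Spawnfence spawns them, sends each a false visibility message and stores them in MyKids.
; ChildStopThinking destroys them, with paired DoOnce nodes re-arming each other so start and stop alternate.
; Spline mesh building code remains unwired, and the construction script is empty.
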(event `self.ChildStartThinking`
  (`/Engine/EditorBlueprintResources/StandardMacros.DoOnce` false :!label _label
    (:`Completed`
      (`|ExecutionSequence` :!label _label_2
        (:`then_0`
          (goto _label_3 :!via `Reset`))
        (:`then_1`
          (`KismetSystemLibrary.PrintString` "SPAWN BLUEPRINTS")
          (for _index (range (`KismetMathLibrary.FTrunc` (/ (`SplineComponent.GetSplineLength` (`self.Spline`)) (`self.Section Length`))))
            (set `self.LoopIndex` _index)
            (bind (_position _tangent) (`self.GetStartPos/Tan` (`self.LoopIndex`)))
            (bind _returnvalue (`|SpawnActorFromClass` (`self.Class`) (`KismetMathLibrary.MakeTransform` _position (`KismetMathLibrary.Conv_VectorToRotator` _tangent)) "AlwaysSpawn" "MultiplyWithRoot" null null))
            (message `/Game/LeastOfThese/BluePrints/levelStuff/Triggers/BPI_InWorldCommunication.Visibility` _returnvalue false)
            (`KismetArrayLibrary.Array_Add` (`self.MyKids`) _returnvalue)))))))

(event `Spawn fence`
  (goto _label_2))

(event `self.ChildStopThinking`
  (`/Engine/EditorBlueprintResources/StandardMacros.DoOnce` false :!label _label_3
    (:`Completed`
      (`|ExecutionSequence`
        (:`then_0`
          (goto _label :!via `Reset`))
        (:`then_1`
          ; Lol Dark humor
          (`self.K2_DestroyActor` (`self.MyKids`)))))))

(fn `Activate`
  (returns (Successful :type Boolean))
  (return true))

(fn `GetendPos/Tan`
  (params (Index :type Integer))
  (returns (Position :type "Vector Structure") (Tangent :type "Vector Structure") (Scale :type "Vector Structure"))
  (bind _spline (`self.Spline`))
  (bind _returnvalue (* (+ Index 1) (`self.Section Length`)))
  (return (`SplineComponent.GetLocationAtDistanceAlongSpline` _spline _returnvalue "Local") (`KismetMathLibrary.ClampVectorSize` (`SplineComponent.GetTangentAtDistanceAlongSpline` _spline _returnvalue "Local") 0.0 (`self.Section Length`)) (`SplineComponent.GetScaleAtDistanceAlongSpline` _spline _returnvalue)))

(fn `GetStartPos/Tan`
  (params (Index :type Integer))
  (returns (Position :type "Vector Structure") (Tangent :type "Vector Structure") (Scale :type "Vector Structure"))
  (bind _spline (`self.Spline`))
  (bind _returnvalue (* Index (`self.Section Length`)))
  (return (`SplineComponent.GetLocationAtDistanceAlongSpline` _spline _returnvalue "World") (`KismetMathLibrary.ClampVectorSize` (`SplineComponent.GetTangentAtDistanceAlongSpline` _spline _returnvalue "World") 0.0 (`self.Section Length`)) (`SplineComponent.GetScaleAtDistanceAlongSpline` _spline _returnvalue)))

(fn `UserConstructionScript`)