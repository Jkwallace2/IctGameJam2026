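; BP_ExplodingCrate is a crate that sets off an explosion when it breaks.
; The PreBreak event passes through a DoOnce gate, so the sequence runs a single time.
; It waits a tick, spawns BP_Explosion at the crate's location, then waits another tick before calling Breakdown.
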(event `self.PreBreak`
  (`/Engine/EditorBlueprintResources/StandardMacros.DoOnce` false
    (:`Completed`
      (`KismetSystemLibrary.DelayUntilNextTick`)
      (`|SpawnActorFromClass` "/Game/LeastOfThese/BluePrints/Explosions/BP_Explosion.BP_Explosion_C" (`KismetMathLibrary.Conv_VectorToTransform` (`self.K2_GetActorLocation`)) "Undefined" "MultiplyWithRoot" null null null)
      (`KismetSystemLibrary.DelayUntilNextTick`)
      (`self.Breakdown`))))

(fn `UserConstructionScript`
  (`parent.UserConstructionScript`))