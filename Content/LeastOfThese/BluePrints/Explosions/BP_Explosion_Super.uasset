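; Super explosion actor that stages a nuke-style blast with global slow motion, then destroys itself.
; BeginPlay sends a full-radius damage message and noise, overrides submix effects, and runs a time-dilation timeline into ShockWave.
; ShockWave expands a sphere trace, mesh and white camera fade, damaging each new actor once, sparing the player and trigger boards/marbles.
; Reaching the player, or finishing, triggers force feedback, the delayed boom and time-dilation recovery.
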(event `self.ReceiveBeginPlay`
  (bind _origin (`self.Origin`))
  ; explosion
  (bind _outactors (`GameplayStatics.GetAllActorsOfClass` "/Game/LeastOfThese/BluePrints/levelStuff/Triggers/BP_TrigBoard_KU.BP_TrigBoard_KU_C"))
  (set `self.Actors to Ignore` _outactors)
  (bind _outactors_2 (`GameplayStatics.GetAllActorsOfClass` "/Game/LeastOfThese/BluePrints/levelStuff/Triggers/BP_TrigMarble_DK.BP_TrigMarble_DK_C"))
  (for _array_element _outactors_2
    (`KismetArrayLibrary.Array_Add` (`self.Actors to Ignore`) _array_element))
  (`GameplayStatics.PlaySound2D` "/Game/Audio/SFX/WallaceToySFX/03_Bells/Bell_Crowbar_Reversed.Bell_Crowbar_Reversed" 1.0 1.0 0.8 null null)
  (`GameplayStatics.PlaySound2D` "/Game/Audio/SFX/SawSaber.SawSaber" 1.0 1.0 0.0 null null)
  (bind _output_get (set `self.Origin` (`SceneComponent.K2_GetComponentLocation` (`self.DefaultSceneRoot`))))
  (`self.MakeNoise` 3.0 (`GameplayStatics.GetPlayerPawn` 0) _output_get)
  (`NiagaraFunctionLibrary.SpawnSystemAtLocation` "/Game/LeastOfThese/VFX/NS_HelperSuper.NS_HelperSuper" _output_get)
  (bind _outhits (`KismetSystemLibrary.SphereTraceMultiForObjects` _origin _origin (`self.DamageRadius`) (`self.Object Types_0`)))
  (for _array_element_2 _outhits
    (bind (_bblockinghit _binitialoverlap _time _distance _location _impactpoint _normal _impactnormal _physmat _hitactor) (`GameplayStatics.BreakHitResult` _array_element_2))
    (message `/Game/LeastOfThese/BluePrints/GameSystems/ToyPhisANdDamage/BPI_ToyDamage.LotDamage` _hitactor "NewEnumerator0" 0 (* _normal 1.0) (`GameplayStatics.GetPlayerController` 0) self 0 0 _location)
    (`KismetArrayLibrary.Array_Add` (`self.FinalHits`) _array_element_2))
  (`AudioMixerBlueprintLibrary.SetSubmixEffectChainOverride` "/Engine/EngineSounds/Submixes/MasterSubmixDefault.MasterSubmixDefault" (`self.Submix Effect Preset Chain`) 0.1)
  (`AddComponent|NODE_AddAudioComponent-1`)
  (bind (_direction _newtrack_0) (`Timeline|Timeline_0`)
    (:`Update`
      (`GameplayStatics.SetGlobalTimeDilation` (`KismetMathLibrary.MapRangeClamped` _newtrack_0 0.0 1.0 1.0 0.1)))
    (:`Finished`
      (`self.ShockWave`))))

(event `ShockWave`
  (bind _returnvalue (`GameplayStatics.GetPlayerController` 0))
  (bind _returnvalue_2 (`SceneComponent.K2_GetComponentLocation` (`self.DefaultSceneRoot`)))
  (bind _returnvalue_3 (`KismetMathLibrary.FTrunc` (`KismetMathLibrary.MapRangeClamped` (* (`self.I`) 0.01) 1.0 0.0 1.0 5.0)))
  ; explosion
  ;; Shockwave
  (`/Engine/EditorBlueprintResources/StandardMacros.DoOnce` false
    (:`Completed`
      (bind (_direction _newtrack_0) (`Timeline|Timeline` :!via `PlayFromStart`)
        (:`Update`
          (`PlayerCameraManager.SetManualCameraFade` (`PlayerController.PlayerCameraManager` (`GameplayStatics.GetPlayerController` 0)) (`KismetMathLibrary.FClamp` (- 1.0 _newtrack_0)) (struct :`R` 1.0 :`G` 1.0 :`B` 1.0 :`A` 1.0) true)
          (bind _output_get (set `self.I` _newtrack_0))
          (`SceneComponent.K2_SetRelativeLocation` (`self.PointLight`) (`KismetMathLibrary.VLerp` (0.0 0.0 0.0) (0.0 0.0 5000.0) _output_get) false true)
          (bind _returnvalue_4 (`KismetMathLibrary.Lerp` 0.0 (`self.DamageRadius`) _output_get))
          (`SceneComponent.SetWorldScale3D` (`self.Sphere1`) (`KismetMathLibrary.Conv_DoubleToVector` (* _returnvalue_4 1.2)))
          (bind _outhits (`KismetSystemLibrary.SphereTraceMultiForObjects` _returnvalue_2 _returnvalue_2 _returnvalue_4 (`self.Object Types_0`) false (`self.Actors to Ignore`)))
          (for _array_element _outhits
            (bind (_bblockinghit _binitialoverlap _time _distance _location _impactpoint _normal _impactnormal _physmat _hitactor) (`GameplayStatics.BreakHitResult` _array_element))
            (`KismetArrayLibrary.Array_Add` (`self.Actors to Ignore`) _hitactor)
            (`KismetSystemLibrary.IsObjectOfSoftClass` _hitactor "/Game/LeastOfThese/BluePrints/GameSystems/AI/Parents/BP_LOTEnemy.BP_LOTEnemy_C"
              (:`True`
                (bind _returnvalue_5 (* _normal 1.0))
                (message `/Game/LeastOfThese/BluePrints/GameSystems/ToyPhisANdDamage/BPI_ToyDamage.LotDamage` _hitactor "NewEnumerator0" _returnvalue_3 _returnvalue_5 _returnvalue self 0 0 _location "NewEnumerator1"))
              (:`False`
                (`KismetSystemLibrary.IsObjectOfSoftClass` _hitactor "/Game/StateTreePlayer/FirstPerson/Blueprints/BP_StateTreePlayer.BP_StateTreePlayer_C"
                  (:`True`
                    (`/Engine/EditorBlueprintResources/StandardMacros.DoOnce` false
                      (:`Completed`
                        (set `self.FoundPlayer` true)
                        (`self.PlayerSound`))))
                  (:`False`
                    (message `/Game/LeastOfThese/BluePrints/GameSystems/ToyPhisANdDamage/BPI_ToyDamage.LotDamage` _hitactor "NewEnumerator0" _returnvalue_3 _returnvalue_5 _returnvalue self 0 0 (0.0 0.0 0.0) "NewEnumerator2")))))))
        (:`Finished`
          (`GameplayStatics.SetGlobalTimeDilation` 1.0)
          (if (not (`self.FoundPlayer`))
            (`self.PlayerSound`)))))))

(event `PlayerSound`
  (`GameplayStatics.SpawnForceFeedbackAtLocation` "/Game/LeastOfThese/BluePrints/Explosions/FFE_Nuke.FFE_Nuke" (`self.Origin`) (struct) false 1.0 0.0 null)
  (`AudioMixerBlueprintLibrary.ClearSubmixEffectChainOverride` "/Engine/EngineSounds/Submixes/MasterSubmixDefault.MasterSubmixDefault")
  (`GameplayStatics.PlaySound2D` "/Game/Audio/Bombs/NukeInstant.NukeInstant" 1.0 1.0 0.0 null null)
  (bind (_direction _newtrack_0) (`Timeline|Timeline_1`)
    (:`Update`
      (`GameplayStatics.SetGlobalTimeDilation` _newtrack_0))
    (:`Finished`
      (`self.K2_DestroyActor`))))

(fn `AreYouUsingToyPhys`
  (returns (Yeah :type Boolean))
  (return false))

(fn `UserConstructionScript`
  (`SphereComponent.SetSphereRadius` (`self.Sphere`) (`self.DamageRadius`) true))

(fn `WhatIsYourWeight`
  (returns (Weight :type "/Game/LeastOfThese/BluePrints/GameSystems/ToyPhisANdDamage/E_ToyWeight_MOVEDFORMIGRATION_4 Enum"))
  (return "NewEnumerator0"))