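; Nuke explosion actor that mutes SFX, slows global time, spawns the blast effect and makes noise on BeginPlay.
; A deduplicated sphere trace, line-checked for occlusion, applies point damage, evaporates enemies and pushes physics objects.
; After a short delay, Tick expands a damaging shockwave while the light rises and fades.
; Boom, rumble and SFX restore wait until the wave reaches the player or ends, when time resets and the actor destroys itself.
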(event `self.ReceiveBeginPlay`
  (bind _origin (`self.Origin`))
  ; explosion
  (`GameplayStatics.SetSoundMixClassOverride` null "/Engine/EngineSounds/SFX.SFX" 0.0 1.0 0.0)
  (`GameplayStatics.SetGlobalTimeDilation` 0.1)
  (set `self.Intensity` (`LightComponentBase.Intensity` (`self.PointLight`)))
  (bind _output_get (set `self.Origin` (`SceneComponent.K2_GetComponentLocation` (`self.DefaultSceneRoot`))))
  (`self.MakeNoise` 3.0 (`GameplayStatics.GetPlayerPawn` 0) _output_get)
  (`NiagaraFunctionLibrary.SpawnSystemAtLocation` "/Game/LeastOfThese/VFX/NS_Nuke.NS_Nuke" _output_get)
  (bind _outhits (`KismetSystemLibrary.SphereTraceMultiByProfile` _origin _origin (`self.DamageRadius`) "BlockAll"))
  ;; There are multiple hits per actor, include each actor once
  (for _array_element _outhits
    (bind (_bblockinghit _binitialoverlap _time _distance _location _impactpoint _normal _impactnormal _physmat _hitactor) (`GameplayStatics.BreakHitResult` _array_element))
    (if (`KismetArrayLibrary.Array_Contains` (`self.Array Element Hit Actor`) _hitactor)
      (`self.ShockWave`)
      (else
        (`KismetArrayLibrary.Array_Add` (`self.Array Element Hit Actor`) _hitactor)
        (`KismetArrayLibrary.Array_Add` (`self.GoodHits`) _array_element))))
  ;; Explosion Occlusion
  (for _array_element_2 (`self.GoodHits`)
    (bind (_bblockinghit_2 _binitialoverlap_2 _time_2 _distance_2 _location_2 _impactpoint_2 _normal_2 _impactnormal_2 _physmat_2 _hitactor_2) (`GameplayStatics.BreakHitResult` _array_element_2))
    (bind (_outhit _returnvalue) (`KismetSystemLibrary.LineTraceSingleByProfile` (+ _impactpoint_2 (* _normal_2 50.0)) (`self.Origin`) "BlockAll" false (`|MakeArray` _hitactor_2 (`self.Creator`)) "None" true (struct :`R` 0.04883 :`G` 1.0 :`A` 1.0) (struct :`R` 1.0 :`G` 0.064089 :`A` 1.0)))
    ;;; If the is no blocking hit, then the explosion got us. using aray so occlusion still works.
    (if (not _returnvalue)
      (`KismetArrayLibrary.Array_Add` (`self.FinalHits`) _array_element_2)))
  (if (> (`KismetArrayLibrary.Array_Length` (`self.FinalHits`)) 0)
    ;; Damage
    (for _array_element_3 (`self.FinalHits`)
      (`self.DagageCharacters` _array_element_3)
      (`self.Impulse Physics` _array_element_3)
      (bind (_bblockinghit_3 _binitialoverlap_3 _time_3 _distance_3 _location_3 _impactpoint_3 _normal_3 _impactnormal_3 _physmat_3 _hitactor_3 _hitcomponent _hitbonename _bonename _hititem _elementindex _faceindex _tracestart _traceend) (`GameplayStatics.BreakHitResult` _array_element_3))
      (`GameplayStatics.ApplyPointDamage` _hitactor_3 (`KismetMathLibrary.MapRangeClamped` (`KismetMathLibrary.Vector_Distance` _tracestart _traceend) 0.0 (`self.DamageRadius`) 5.0 (`self.Damage`)) _impactnormal_3 _array_element_3 (`self.GetInstigatorController`) (`self.Creator`)))
    (`self.ShockWave`)
    (else
      (`self.ShockWave`))))

(event `ShockWave`
  ; explosion
  ;; Shockwave
  (`/Engine/EditorBlueprintResources/StandardMacros.DoOnce` false
    (:`Completed`
      (set `self.I` 0.0)
      (`KismetSystemLibrary.Delay` 0.1)
      (set `self.Gate` true))))

(event `DagageCharacters`
  (params (hit :type "HitResult Structure"))
  ; explosion
  ;; Unreal thinks this is an infinite loop, but only some times
  ;; Radial Fall off For Character pawns
  (bind _asbp_lotenemy (cast `/Game/LeastOfThese/BluePrints/GameSystems/AI/Parents/BP_LOTEnemy` (`.HitActor` (`GameplayStatics.BreakHitResult` hit))))
  (`/Game/LeastOfThese/BluePrints/GameSystems/AI/Parents/BP_Creature.Evaporate` _asbp_lotenemy))

(event `self.ReceiveTick`
  (params (DeltaSeconds :type "Float (single-precision)"))
  (bind _object_types (`self.Object Types`))
  (bind _returnvalue (`SceneComponent.K2_GetComponentLocation` (`self.DefaultSceneRoot`)))
  ; explosion
  ;; Shockwave
  (if (`self.Gate`)
    (bind _output_get (set `self.I` (`KismetMathLibrary.FInterpTo_Constant` (`self.I`) 1.0 DeltaSeconds 1.0)))
    (if (== (`self.I`) 1.0)
      (`GameplayStatics.SetGlobalTimeDilation` 1.0)
      (if (not (`self.FoundPlayer`))
        (`self.PlayerSound`))
      (`self.K2_DestroyActor`)
      (else
        (`LightComponent.SetIntensity` (`self.PointLight`) (`KismetMathLibrary.Lerp` (`self.Intensity`) 0.0 _output_get))
        (`SceneComponent.K2_SetRelativeLocation` (`self.PointLight`) (`KismetMathLibrary.VLerp` (0.0 0.0 0.0) (0.0 0.0 2000.0) _output_get) false true)
        (bind _returnvalue_2 (* _output_get 13000.0))
        (bind (_outactors _returnvalue_3) (`KismetSystemLibrary.SphereOverlapActors` _returnvalue _returnvalue_2 _object_types "/Game/StateTreePlayer/FirstPerson/Blueprints/BP_StateTreePlayer.BP_StateTreePlayer_C"))
        (`|ExecutionSequence`
          (:`then_0`
            (bind _outhits (`KismetSystemLibrary.SphereTraceMultiForObjects` _returnvalue _returnvalue (`KismetMathLibrary.FClamp` _returnvalue_2 0.0 8000.0) _object_types))
            (for _array_element _outhits
              (bind (_bblockinghit _binitialoverlap _time _distance _location _impactpoint _normal _impactnormal _physmat _hitactor) (`GameplayStatics.BreakHitResult` _array_element))
              (if (!= _hitactor (`GameplayStatics.GetPlayerPawn` 0))
                (bind _returnvalue_4 (* _normal -1.0))
                (`GameplayStatics.ApplyPointDamage` _hitactor (`self.Damage`) _returnvalue_4 _array_element null (`self.Creator`))
                (message `/Game/LeastOfThese/BluePrints/GameSystems/ToyPhisANdDamage/BPI_ToyDamage.LotDamage` _hitactor "NewEnumerator0" 3 _returnvalue_4 null self 0 0 (0.0 0.0 0.0)))))
          (:`then_1`
            (if _returnvalue_3
              (`/Engine/EditorBlueprintResources/StandardMacros.DoOnce` false
                (:`Completed`
                  (set `self.FoundPlayer` true)
                  (`self.PlayerSound`))))))))))

(event `PlayerSound`
  ; explosion
  (`GameplayStatics.PlaySound2D` "/Game/Audio/Bombs/SC_Nuke_Cue.SC_Nuke_Cue" 3.0 1.0 0.0 null null)
  (`GameplayStatics.SpawnForceFeedbackAtLocation` "/Game/LeastOfThese/BluePrints/Explosions/FFE_Nuke.FFE_Nuke" (`self.Origin`) (struct) false 1.0 0.0 null)
  (`GameplayStatics.SetSoundMixClassOverride` null "/Engine/EngineSounds/SFX.SFX" 1.0 1.0 2.0))

(event `Impulse Physics`
  (params (hit :type "HitResult Structure"))
  ; explosion
  ;; impulse for physics objects
  (`PrimitiveComponent.AddRadialForce` (`.HitComponent` (`GameplayStatics.BreakHitResult` hit)) (- (`self.K2_GetActorLocation`) (0.0 0.0 50.0)) (`self.DamageRadius`) (* (`self.KnockBack`) 30.0) "RIF_Linear" true))

(fn `AreYouUsingToyPhys`
  (returns (Yeah :type Boolean))
  (return false))

(fn `UserConstructionScript`
  (`SphereComponent.SetSphereRadius` (`self.Sphere`) (`self.DamageRadius`) true))

(fn `WhatIsYourWeight`
  (returns (Weight :type "/Game/LeastOfThese/BluePrints/GameSystems/ToyPhisANdDamage/E_ToyWeight_MOVEDFORMIGRATION_4 Enum"))
  (return "NewEnumerator0"))