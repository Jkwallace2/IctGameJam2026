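; Crouching state in the player's state machine, handling uncrouch, jump and kicks while crouched.
; Releasing crouch or pressing jump switches to another state, gated by the player's CyoteStep check.
; Forward and idle kicks zero ground friction and braking, add a clamped dodge-speed impulse, then run the basic forward kick, producing a sliding lunge.
; Losing ground calls CrouchAny before parent handling; bhop-slide buffer and camera-crouch calls on enter are disconnected.
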(event `self.TryCrouch`
  (params (Active :type Boolean) (Anolouge :type Boolean) (Trigger :type "Float (double-precision)"))
  (if (not Active)
    (if (`/Game/StateTreePlayer/FirstPerson/Blueprints/BP_StateTreePlayer.CyoteStep` (`self.Player`)) :!label _label
      (`self.SwitchState` "NewEnumerator1"))))

(event `self.TryJump`
  (params (True :type Boolean))
  (goto _label))

(event `self.ChildForwardKick`
  (params (Kick :type "/Game/LeastOfThese/DataTables/Structures/Struct_Kick Structure"))
  (bind _charactermovement (`Character.CharacterMovement` (`self.Player`)))
  (set `CharacterMovementComponent.GroundFriction` 0.0 _charactermovement)
  (set `CharacterMovementComponent.BrakingDecelerationWalking` 0.0 _charactermovement)
  (bind _newvelocity (`self.ClampVelocitytoAdd` (`self.DodgeSpeed`)))
  (`CharacterMovementComponent.AddImpulse` (`Character.CharacterMovement` (`self.Player`)) _newvelocity true)
  (`self.BasicForwardKick` Kick))

(event `self.ChildIdleKick`
  (params (Kick :type "/Game/LeastOfThese/DataTables/Structures/Struct_Kick Structure"))
  (bind _charactermovement (`Character.CharacterMovement` (`self.Player`)))
  (set `CharacterMovementComponent.GroundFriction` 0.0 _charactermovement)
  (set `CharacterMovementComponent.BrakingDecelerationWalking` 0.0 _charactermovement)
  (bind _newvelocity (`self.ClampVelocitytoAdd` (`self.DodgeSpeed`)))
  (`CharacterMovementComponent.AddImpulse` (`Character.CharacterMovement` (`self.Player`)) _newvelocity true)
  (`self.BasicForwardKick` Kick))

(fn `Crouchtokick`)

(fn `NoLongerOnGround`
  (`self.CrouchAny`)
  (`parent.NoLongerOnGround`))

(fn `OldDodge`)

(fn `OnEnter`
  (`parent.OnEnter`))