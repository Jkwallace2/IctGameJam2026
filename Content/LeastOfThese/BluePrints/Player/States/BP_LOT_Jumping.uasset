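; Player state for jumping: on enter it applies an upward impulse sized for the jump height, clears coyote step and enables ground pound.
; A forward or idle kick fires once, estimating height gained from velocity loss and relaunching toward knee-kick height.
; A back kick adds upward impulse for a backflip.
; Crouch presses hand off to CrouchAny, and both ground-contact changes call StandAny.
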(event `self.TryCrouch`
  (params (Active :type Boolean) (Anolouge :type Boolean) (Trigger :type "Float (double-precision)"))
  ; only if pressed down
  (if Active
    (`self.CrouchAny`)))

(event `self.ChildIdleKick`
  (params (Kick :type "/Game/LeastOfThese/DataTables/Structures/Struct_Kick Structure"))
  (`self.ChildForwardKick` Kick))

(event `self.ChildForwardKick`
  (params (Kick :type "/Game/LeastOfThese/DataTables/Structures/Struct_Kick Structure"))
  (bind (_returnvalue_x _returnvalue_y _returnvalue_z) (`KismetMathLibrary.BreakVector` (`CharacterMovementComponent.GetLastUpdateVelocity` (`Character.CharacterMovement` (`self.Player`)))))
  (bind _returnvalue (/ (- (`KismetMathLibrary.Square` (`self.EnterJumpVelocity`)) (`KismetMathLibrary.Square` _returnvalue_z)) (* 2.0 980.0)))
  (if (not (`self.DidKick`))
    (`/Engine/EditorBlueprintResources/StandardMacros.DoOnce` false
      (:`Completed`
        (`|ExecutionSequence`
          (:`then_0`
            (`KismetSystemLibrary.PrintString` null (`KismetStringLibrary.Conv_DoubleToString` _returnvalue) true true (struct :`R` 1.0 :`G` 0.56753 :`A` 1.0))
            (`Character.LaunchCharacter` (`self.Player`) (`KismetMathLibrary.MakeVector` 0.0 0.0 (`/Game/StateTreePlayer/FirstPerson/Blueprints/BP_StateTreePlayer.CalculateJumpVelocity` (`self.Player`) (- (`/Game/StateTreePlayer/FirstPerson/Blueprints/BP_StateTreePlayer.KneeKickHeight` (`self.Player`)) _returnvalue))) false true)
            (set `self.DidKick` true)
            (`/Game/StateTreePlayer/FirstPerson/Blueprints/BP_StateTreePlayer.SuperJumpSound` (`self.Player`)))
          (:`then_1`
            (`self.BasicForwardKick` Kick)
            (`/Game/StateTreePlayer/FirstPerson/Blueprints/BP_StateTreePlayer.openKickGate` (`self.Player`))))))))

(event `self.ChildBackKick`
  (params (Kick :type "/Game/LeastOfThese/DataTables/Structures/Struct_Kick Structure"))
  ; BackFlip
  (`CharacterMovementComponent.AddImpulse` (`Character.CharacterMovement` (`self.Player`)) (* (`KismetMathLibrary.MakeVector` 0.0 0.0 (`.VelocityIfApplicable_30_D292BA0741750075448518972CBA720B` (break `/Game/LeastOfThese/DataTables/Structures/Struct_Kick` Kick))) (`/Game/StateTreePlayer/FirstPerson/Blueprints/BP_StateTreePlayer.JumpHeight` (`self.Player`))) true)
  (`self.BasicForwardKick` Kick)
  (`/Game/StateTreePlayer/FirstPerson/Blueprints/BP_StateTreePlayer.BackFlipTest` (`self.Player`))
  (`/Game/StateTreePlayer/FirstPerson/Blueprints/BP_StateTreePlayer.openKickGate` (`self.Player`)))

(fn `NoLongerOnGround`
  (`self.StandAny`)
  (`parent.NoLongerOnGround`))

(fn `NowOnGround`
  (`self.StandAny`)
  (`parent.NowOnGround`))

(fn `OnEnter`
  (bind _player (`self.Player`))
  (`parent.OnEnter`)
  (set `self.EnterJumpVelocity` (`/Game/StateTreePlayer/FirstPerson/Blueprints/BP_StateTreePlayer.CalculateJumpVelocity` _player (`/Game/StateTreePlayer/FirstPerson/Blueprints/BP_StateTreePlayer.JumpHeight` _player)))
  (set `/Game/StateTreePlayer/FirstPerson/Blueprints/BP_StateTreePlayer.CanGroundPound` true (`self.Player`))
  (set `/Game/StateTreePlayer/FirstPerson/Blueprints/BP_StateTreePlayer.CyoteStep` false (`self.Player`))
  (`CharacterMovementComponent.AddImpulse` (`Character.CharacterMovement` (`self.Player`)) (* (0.0 0.0 1.0) (`self.EnterJumpVelocity`)) true))