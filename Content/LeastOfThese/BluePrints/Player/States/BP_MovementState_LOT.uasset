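; Base player movement state that gives each state its own directional kicks and kick animations.
; On enter it loads kick and animation rows by StateRow, then opens the player's kick gate unless a kick-on-entry is pending.
; Kick events play the animation and call overridable Child events, with left and right sharing Side data via a mirrored offset.
; The default Basic kick functions are stubs.
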(event `LeftKick_1`
  (params (Down :type Boolean))
  (bind (_toytype _power _range _sweep _l_roffset _box _animation_test _velocityifapplicable) (break `/Game/LeastOfThese/DataTables/Structures/Struct_Kick` (`.Side_7_FD6EDB9C446CBEB52A6DED93BFE1D3A7` (break `/Game/LeastOfThese/DataTables/Structures/Struct_StateKicks` (`self.StateKicks`)))))
  (`/Game/StateTreePlayer/FirstPerson/Blueprints/BP_StateTreePlayer.KickAnim` (`self.Player`) (`.Right_14_46749BD5458A128DECF496A47F1E3E5B` (break `/Game/LeastOfThese/DataTables/Structures/Struct_StateAnims` (`self.StateAnim`))))
  (`self.ChildLeftKick` (make `/Game/LeastOfThese/DataTables/Structures/Struct_Kick` _toytype _power _range _sweep (* _l_roffset -1.0) _box null _velocityifapplicable)))

(event `IdleKick_1`
  (params (Down :type Boolean))
  (`/Game/StateTreePlayer/FirstPerson/Blueprints/BP_StateTreePlayer.KickAnim` (`self.Player`) (`.Idle_8_2C61580343FF8900A56247B31AC321F8` (break `/Game/LeastOfThese/DataTables/Structures/Struct_StateAnims` (`self.StateAnim`))))
  (`self.ChildIdleKick` (`.Idle_2_93D7316C486FD1FC3E58AEAAD1984FD0` (break `/Game/LeastOfThese/DataTables/Structures/Struct_StateKicks` (`self.StateKicks`)))))

(event `ForwardKick_1`
  (params (Down :type Boolean))
  (`/Game/StateTreePlayer/FirstPerson/Blueprints/BP_StateTreePlayer.KickAnim` (`self.Player`) (`.Forward_9_36A617F14829B9B21CD5B68BBA513334` (break `/Game/LeastOfThese/DataTables/Structures/Struct_StateAnims` (`self.StateAnim`))))
  (`self.ChildForwardKick` (`.Forward_6_45C3468843C9DCE9EF2BE99810B70C77` (break `/Game/LeastOfThese/DataTables/Structures/Struct_StateKicks` (`self.StateKicks`)))))

(event `BackKick_1`
  (params (Down :type Boolean))
  (`/Game/StateTreePlayer/FirstPerson/Blueprints/BP_StateTreePlayer.KickAnim` (`self.Player`) (`.Back_11_804565E04C4E4261C6519DAB76BE5DEE` (break `/Game/LeastOfThese/DataTables/Structures/Struct_StateAnims` (`self.StateAnim`))))
  (`self.ChildBackKick` (`.Back_9_5BEAB0DD4989E37DB4A83291F6DB0D22` (break `/Game/LeastOfThese/DataTables/Structures/Struct_StateKicks` (`self.StateKicks`)))))

(event `RightKick_1`
  (params (Down :type Boolean))
  (bind (_toytype _power _range _sweep _l_roffset _box _animation_test _velocityifapplicable) (break `/Game/LeastOfThese/DataTables/Structures/Struct_Kick` (`.Side_7_FD6EDB9C446CBEB52A6DED93BFE1D3A7` (break `/Game/LeastOfThese/DataTables/Structures/Struct_StateKicks` (`self.StateKicks`)))))
  (`/Game/StateTreePlayer/FirstPerson/Blueprints/BP_StateTreePlayer.KickAnim` (`self.Player`) (`.Left_13_B78C8E3A45221B6390B8D6A372C0880B` (break `/Game/LeastOfThese/DataTables/Structures/Struct_StateAnims` (`self.StateAnim`))))
  (`self.ChildRightKick` (make `/Game/LeastOfThese/DataTables/Structures/Struct_Kick` _toytype _power _range _sweep _l_roffset _box null _velocityifapplicable)))

(event `ChildForwardKick`
  (params (Kick :type "/Game/LeastOfThese/DataTables/Structures/Struct_Kick Structure"))
  ; Children will override if they do something special
  (`self.BasicForwardKick` Kick))

(event `ChildIdleKick`
  (params (Kick :type "/Game/LeastOfThese/DataTables/Structures/Struct_Kick Structure"))
  ; Children will override if they do something special
  (`self.BasicForwardKick` Kick))

(event `ChildRightKick`
  (params (Kick :type "/Game/LeastOfThese/DataTables/Structures/Struct_Kick Structure"))
  ; Children will override if they do something special
  (`self.BasicSideKick` Kick))

(event `ChildLeftKick`
  (params (Kick :type "/Game/LeastOfThese/DataTables/Structures/Struct_Kick Structure"))
  ; Children will override if they do something special
  (`self.BasicSideKick` Kick))

(event `ChildBackKick`
  (params (Kick :type "/Game/LeastOfThese/DataTables/Structures/Struct_Kick Structure"))
  ; Children will override if they do something special
  (`self.BasicForwardKick` Kick))

(fn `BasicForwardKick`
  (params (Struct_Kick :type "/Game/LeastOfThese/DataTables/Structures/Struct_Kick Structure (by ref)"))
  (returns (DidHit :type Boolean))
  (`KismetSystemLibrary.PrintString` null "BasicForwardKick")
  (return false))

(fn `BasicSideKick`
  (params (Kick :type "/Game/LeastOfThese/DataTables/Structures/Struct_Kick Structure")))

(fn `OnEnter`
  (bind _player (`self.Player`))
  (bind _returnvalue (`|GetDataTableRow` (`self.KickSheet`) (`self.State Row`))
    (:`then`
      (set `self.StateKicks` _returnvalue)
      (bind _returnvalue_2 (`|GetDataTableRow` (`self.AnimationSheet`) (`self.State Row`))
        (:`then`
          (set `self.StateAnim` _returnvalue_2)
          (if (not (and (`/Game/StateTreePlayer/FirstPerson/Blueprints/BP_StateTreePlayer.KickOnStateEntered` _player) (`/Game/StateTreePlayer/FirstPerson/Blueprints/BP_StateTreePlayer.WantToKick` _player)))
            (`/Game/StateTreePlayer/FirstPerson/Blueprints/BP_StateTreePlayer.openKickGate` _player)
            (`/Game/StateTreePlayer/FirstPerson/Blueprints/BP_StateTreePlayer.openKickGate` (`self.Player`))
            (`parent.OnEnter` :!label _label)))
        (:`RowNotFound`
          (`KismetSystemLibrary.PrintString` null "KICK ANIMATION DATA NOT FOUND" true true (struct :`R` 1.0 :`G` 0.004868 :`A` 1.0) 5.0)
          (goto _label))))
    (:`RowNotFound`
      (`KismetSystemLibrary.PrintString` null "KICK TABLE DATA NOT FOUND" true true (struct :`R` 1.0 :`G` 0.004868 :`A` 1.0) 5.0)
      (goto _label))))