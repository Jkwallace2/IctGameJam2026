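; Player state for crouching while airborne, part of the LeastOfThese player state set.
; Pressing jump or releasing crouch calls StandAny, and landing switches to another state before running the parent landing logic.
; DK_LOM2 launches the player backward and slightly upward with a velocity impulse.
; Camera crouch and a dropkick ground pound on landing are disconnected, and OldDodge and Crouchtokick are empty.
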(event `self.TryJump`
  (params (True :type Boolean))
  (`self.StandAny` :!label _label))

(event `self.TryCrouch`
  (params (Active :type Boolean) (Anolouge :type Boolean) (Trigger :type "Float (double-precision)"))
  (if (not Active)
    (goto _label)))

(fn `Crouchtokick`)

(fn `DK_LOM2`
  (bind _player (`self.Player`))
  (`CharacterMovementComponent.AddImpulse` (`Character.CharacterMovement` _player) (+ (* (`Actor.GetActorForwardVector` _player) -1000) (0.0 0.0 200.0)) true) ; Stop
)

(fn `NowOnGround`
  (`self.SwitchState` "NewEnumerator4")
  (`parent.NowOnGround`))

(fn `OldDodge`)

(fn `OnEnter`
  (`parent.OnEnter`))