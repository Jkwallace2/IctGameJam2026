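; Player state for being airborne, part of a state-based player controller.
; A crouch press calls CrouchAny, while a release calls BeginPlay; landing calls StandAny and then the parent's landing logic.
; State entry only runs the parent's logic, as the camera uncrouch is disconnected.
; The back-kick event is empty, with its WebsterKick sound, gate and recoil/lift impulse logic left unwired.
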(event `self.TryCrouch`
  (params (Active :type Boolean) (Anolouge :type Boolean) (Trigger :type "Float (double-precision)"))
  ; only if pressed down
  (if Active
    (`self.CrouchAny`)
    (else
      (`self.BeginPlay`))))

(event `self.ChildBackKick`
  (params (Kick :type "/Game/LeastOfThese/DataTables/Structures/Struct_Kick Structure"))
  ; WebsterKick
)

(fn `NowOnGround`
  (`self.StandAny`)
  (`parent.NowOnGround`))

(fn `OnEnter`
  (`parent.OnEnter`))