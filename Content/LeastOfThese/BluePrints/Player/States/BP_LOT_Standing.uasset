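; Player movement state for standing in the LeastOfThese game, one of the states the player switches between.
; A jump request switches to another state while the player's coyote-time flag is set, and a crouch press triggers crouching.
; Leaving the ground calls a stand helper before the parent handler.
; Entry only runs the parent logic, as the buffered-jump, bhop-slide and camera uncrouch nodes are disconnected.
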(event `self.TryJump`
  (params (True :type Boolean))
  (if (`/Game/StateTreePlayer/FirstPerson/Blueprints/BP_StateTreePlayer.CyoteStep` (`self.Player`))
    (`self.SwitchState` "NewEnumerator1")))

(event `self.TryCrouch`
  (params (Active :type Boolean) (Anolouge :type Boolean) (Trigger :type "Float (double-precision)"))
  ; only if pressed down
  (if Active
    (`self.CrouchAny`)
    (else
      (`self.BeginPlay`) ; ???? What, what does this do?
    )))

(fn `NoLongerOnGround`
  (`self.StandAny`)
  (`parent.NoLongerOnGround`))

(fn `OnEnter`
  (`parent.OnEnter`))