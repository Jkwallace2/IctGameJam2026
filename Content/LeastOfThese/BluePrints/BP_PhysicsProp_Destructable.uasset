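; Destructible physics prop that breaks from damage or impacts, delegating the work to its BPAutoToyBreaker.
; BeginPlay configures the breaker with the mesh, damage rules, threshold and coin count, then damage and hit events are forwarded to it.
; PreBreak leads to a one-shot Breakdown that calls BreakToy.
; SetPreset applies rules for vase, Angry Birds or glass toy types; an older inline damage check remains unconnected.
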(event `self.ReceiveBeginPlay`
  (`parent.ReceiveBeginPlay`)
  (`/Game/LeastOfThese/BluePrints/GameSystems/ToyPhisANdDamage/BP_AutoToyBreaker.SetUpDestructionFX` (`self.BP_AutoToyBreaker`) (`self.StaticMesh`) true (`self.ReciveDamageFrom`) (`self.BreakWhenRecieving`) (`self.MinDamage`) (`self.Coins Count`) 0))

(event `self.ChildLotDmg`
  (params (DamageType :type "/Game/LeastOfThese/BluePrints/GameSystems/ToyPhisANdDamage/E_ToyDamage_MOVEDFORMIGRATION_3 Enum" :default "NewEnumerator0") (Power :type Integer) (Normal :type "Vector Structure") (Location :type "Vector Structure") (ActorThatDidDamage :type "Actor Object Reference"))
  ; DetectDamage
  (`/Game/LeastOfThese/BluePrints/GameSystems/ToyPhisANdDamage/BP_AutoToyBreaker.ProcessToyDamage` (`self.BP_AutoToyBreaker`) Power Normal ActorThatDidDamage))

(event `self.ReceiveHit`
  (params (MyComp :type "PrimitiveComponent Object Reference") (Other :type "Actor Object Reference") (OtherComp :type "PrimitiveComponent Object Reference") (bSelfMoved :type Boolean) (HitLocation :type "Vector Structure") (HitNormal :type "Vector Structure") (NormalImpulse :type "Vector Structure") (Hit :type "HitResult Structure (by ref)"))
  (`/Game/LeastOfThese/BluePrints/GameSystems/ToyPhisANdDamage/BP_AutoToyBreaker.ProcessHit` (`self.BP_AutoToyBreaker`) NormalImpulse Other))

(event `PreBreak`
  (`self.Breakdown`))

(event `Breakdown`
  (`/Engine/EditorBlueprintResources/StandardMacros.DoOnce` false
    (:`Completed`
      (`/Game/LeastOfThese/BluePrints/GameSystems/ToyPhisANdDamage/BP_AutoToyBreaker.BreakToy` (`self.BP_AutoToyBreaker`)))))

(fn `SetPreset`
  (params (Preset :type "/Game/LeastOfThese/BluePrints/GameSystems/ToyPhisANdDamage/E_BreakablePresets Enum" :default "NewEnumerator0"))
  (switch `/Game/LeastOfThese/BluePrints/GameSystems/ToyPhisANdDamage/E_BreakablePresets` Preset
    (:`NewEnumerator0`
      (set `self.ReciveDamageFrom` "NewEnumerator2")
      (set `self.BreakWhenRecieving` "NewEnumerator2")
      (set `self.MinDamage` 0))
    (:`NewEnumerator1`
      (set `self.ReciveDamageFrom` "NewEnumerator2")
      (set `self.BreakWhenRecieving` "NewEnumerator2")
      (set `self.MinDamage` 0)
      (set `self.ToyWeight` "NewEnumerator2"))
    (:`NewEnumerator2`
      (set `self.ReciveDamageFrom` "NewEnumerator0")
      (set `self.BreakWhenRecieving` "NewEnumerator1")
      (set `self.MinDamage` 0))))

(fn `UserConstructionScript`
  (`parent.UserConstructionScript`))